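; StateTree task in the boss AI folder that makes the Pawn wander to a random reachable point within Radius of its current location.
; On arrival it starts a WaitTime timer that calls EndWait, while a failed move finishes the task as failed.
; EndWait randomly sets ShouldJump, then finishes the task successfully.
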(event EventLatentEnterState
  (params (Transition :type State%20Tree%20Transition%20Result%20Structure%20%28by%20ref%29))
  (AI|AIMoveTo (Variables|Default|GetPawn) (.RandomLocation (AI|Navigation|GetRandomReachablePointinRadius (Transformation|GetActorLocation (Variables|Default|GetPawn)) (Variables|Default|GetRadius) 0 0)) 0 5.0 false
    (:OnSuccess
      (Utilities|Time|SetTimerbyFunctionName 0 "EndWait" (Variables|Default|GetWaitTime)))
    (:OnFail
      (StateTree|FinishTask false))))

(fn EndWait
  (Variables|Default|SetshouldJump (Math|Random|RandomBool))
  (StateTree|FinishTask true))