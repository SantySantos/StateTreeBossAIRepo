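; StateTree task for boss AI that tracks whether the AI controller's perception senses the player.
; On entering its state, it binds to the AI Perception component's target perception update event.
; Updates for the player character store that actor and its sensed flag, while other actors clear the stored actor but leave the flag unchanged.
; Each update prints the stored actor's validity for debugging.
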(event EventLatentEnterState
  (params (Transition :type State%20Tree%20Transition%20Result%20Structure%20%28by%20ref%29))
  (CallFunction|CreateBindings))

(fn CreateBindings
  (EventDispatchers|BindEventtoOnTargetPerceptionUpdated (Variables|/Game/STBossesAI/Blueprints/AIC_NPC.AIC_NPC_C|GetAIPerception (Variables|Default|GetAIController)) (EventDispatchers|CreateEvent :!event BindingPerceptionUpdated)))

(fn BindingPerceptionUpdated
  (params (Actor :type Actor%20Object%20Reference) (Stimulus :type AI%20Stimulus%20Structure))
  (bind _returnvalue (Game|GetPlayerCharacter 0))
  (if (== Actor _returnvalue)
    (bind _output_get (Variables|Default|SetActorPerceived _returnvalue))
    (Variables|Default|SetSuccessfully%20Sensed (.bSuccessfullySensed (Utilities|Struct|BreakAIStimulus Stimulus)))
    (Development|PrintString (Utilities|String|ToString(Boolean) (Utilities|IsValid _output_get)))
    (else
      (Variables|Default|SetActorPerceived 0)
      (Development|PrintString (Utilities|String|ToString(Boolean) (Utilities|IsValid _output_get))))))